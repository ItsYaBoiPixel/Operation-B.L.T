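; BP_Tank is a raccoon tank wave enemy that travels along spline paths.
; A looping timeline, paced by Speed, moves Walker along the tutorial, bridge or windy spline, starting automatically only in the tutorial level.
; It increments the wave organizer's active-enemy count on spawn; BustOpen plays the bust effect, decrements it and destroys the actor.
; Its fridge overlap check triggers nothing, and several damage-like leftovers are disconnected.
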(event OnComponentBeginOverlap(BIGCollision)
  (params (OverlappedComponent :type Primitive%20Component%20Object%20Reference) (OtherActor :type Actor%20Object%20Reference) (OtherComp :type Primitive%20Component%20Object%20Reference) (OtherBodyIndex :type Integer) (bFromSweep :type Boolean) (SweepResult :type Hit%20Result%20Structure%20%28by%20ref%29))
  (Utilities|Casting|CastToBP_Fridge OtherActor))

(event Custom|Walk
  (Components|Timeline|SetPlayRate (Variables|Default|GetWalkTimeline) (Variables|Default|GetSpeed))
  (bind _walktrack (Timeline|WalkTimeline PlayFromStart)
    (:Update
      (Transformation|SetWorldLocationAndRotation (Variables|Default|GetWalker) (.location (Spline|GetTransformatDistanceAlongSpline (Variables|Default|GetSplineToFollow) (Math|Float|Lerp 0.0 (Spline|GetSplineLength (Variables|Default|GetSplineToFollow)) _walktrack) "World" false)) (.rotation (Spline|GetTransformatDistanceAlongSpline (Variables|Default|GetSplineToFollow) (Math|Float|Lerp 0.0 (Spline|GetSplineLength (Variables|Default|GetSplineToFollow)) _walktrack) "World" false)) false false))
    (:Finished
      (CallFunction|Walk))))

(event Custom|ComeFromOtherWay
  (Variables|Default|SetComingFromOtherWay true)
  (Variables|Default|SetSplineToFollow (Variables|Default|GetBridgeSpline))
  (CallFunction|Walk))

(event Custom|ComeFromMainWay
  (Variables|Default|SetComingFromOtherWay false)
  (Variables|Default|SetSplineToFollow (Variables|Default|GetWindySpline))
  (CallFunction|Walk))

(event Custom|BustOpen
  (Components|DestroyComponent (Variables|Default|GetRacoonTank))
  (Collision|SetCollisionEnabled (Variables|Default|GetBIGCollision) "NoCollision")
  (Audio|Components|Audio|Play (Variables|Default|GetTankBust) 0.0)
  (Utilities|FlowControl|Delay 1.0)
  (Math|Integer|DecrementInt (Variables|/Game/Blueprints/BP_NewWaveOrganizer.BP_NewWaveOrganizer_C|GetEnemies%20Active (Variables|Default|GetEarlyWaveOragnizer))
    (:%20%20
      (Actor|DestroyActor))))

(event EventBeginPlay
  (Development|PrintText "I exist")
  (Variables|Default|SetSplineToFollow (Variables|Default|GetTutorialSpline))
  (bind _returnvalue (Game|GetCurrentLevelName true))
  (if (Utilities|Enum|Equal(Enum) _returnvalue "Lvl_FInalTutorial")
    (CallFunction|Walk)
    (Development|PrintText "Hello"))
  (bind _outactors (Actor|GetAllActorsOfClass "/Game/Blueprints/BP_NewWaveOrganizer.BP_NewWaveOrganizer_C"))
  (for _array_element _outactors
    (bind _output_get (Variables|Default|SetEarlyWaveOragnizer _array_element))
    (Math|Integer|IncrementInt (Variables|/Game/Blueprints/BP_NewWaveOrganizer.BP_NewWaveOrganizer_C|GetEnemies%20Active (Variables|Default|GetEarlyWaveOragnizer)))))

(event Collision|EventActorBeginOverlap
  (params (OtherActor :type Actor%20Object%20Reference)))

(event EventTick
  (params (DeltaSeconds :type Float%20%28single-precision%29)))

(fn ConstructionScript)