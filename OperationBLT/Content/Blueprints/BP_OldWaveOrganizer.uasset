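; BP_OldWaveOrganizer is an actor that runs timed enemy waves and switches the battle music.
; Tick opens a wave roughly every minute of game time, printing a warning, advancing Wave twice and setting a capped enemy count that grows with it.
; A countdown spaces out BP_Pathway spawns until that count is used up.
; Tick also triggers battle or passive music on an audio component from EnemiesActive, which this Blueprint never updates.
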(event EventBeginPlay
  (bind _returnvalue (AddComponent|AddAudioComponent false))
  (Variables|Default|SetMusicComponent _returnvalue)
  (Variables|Default|SetWave 0))

(event EventTick
  (params (DeltaSeconds :type Float%20%28single-precision%29))
  (bind _wave (Variables|Default|GetWave))
  (bind _musiccomponent (Variables|Default|GetMusicComponent))
  (Variables|Default|SetWait%20Before%20Spawn (- (Variables|Default|GetWait%20Before%20Spawn) DeltaSeconds))
  (if (> (Variables|Default|GetEnemies%20Active) 0)
    (Class|AudioParameterControllerInterface|SetTriggerParameter _musiccomponent "PlayBattle")
    (else
      (Class|AudioParameterControllerInterface|SetTriggerParameter _musiccomponent "PlayPassive")))
  (if (< (Math|Float|%(Float) (Utilities|Time|GetGameTimeinSeconds) 6e+01) 0.1)
    (if (Variables|Default|GetWave%20Active)
      (if (<= (Variables|Default|GetWait%20Before%20Spawn) 0.0) :!label _label
        (if (> (Variables|Default|GetEnemies%20to%20Spawn) 0)
          (Game|SpawnActorfromClass "/Game/Blueprints/BP_Pathway.BP_Pathway_C" (Variables|Default|GetSpawn%20Transform) "Undefined" "MultiplyWithRoot" 0 0)
          (Math|Integer|DecrementInt (Variables|Default|GetEnemies%20to%20Spawn)
            (:%20%20
              (Variables|Default|SetWait%20Before%20Spawn 0.5)))
          (else
            (Variables|Default|SetWave%20Active false))))
      (else
        (Variables|Default|SetWave%20Active true)
        (Math|Integer|IncrementInt (Variables|Default|GetWave)
          (:%20%20
            (Development|PrintText "WAVE INCOMING OH MY GOD")
            (Development|PrintText (Utilities|Text|ToText(Integer) (Variables|Default|GetWave)))
            (Variables|Default|SetEnemies%20to%20Spawn (+ (* _wave 2) 0))
            (Math|Integer|IncrementInt _wave
              (:%20%20
                (if (> (Variables|Default|GetEnemies%20to%20Spawn) 15)
                  (Variables|Default|SetEnemies%20to%20Spawn 15))))))))
    (else
      (goto _label))))

(event Collision|EventActorBeginOverlap
  (params (OtherActor :type Actor%20Object%20Reference)))

(fn ConstructionScript)

(fn NewWave
  (Variables|Default|SetWave%20Active true))