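; BP_Fridge is a fridge actor that loses health when BP_Pathway actors reach its collider.
; On overlap it applies damage to the BP_Pathway actor, subtracts the returned amount from its own FridgeHealth, then destroys that actor.
; Tick pushes FridgeHealth into the FridgeHealthBar widget and rotates the bar to face the player camera.
; Nothing here handles health reaching zero.
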(event OnComponentBeginOverlap(FridgeCollider)
  (params (OverlappedComponent :type Primitive%20Component%20Object%20Reference) (OtherActor :type Actor%20Object%20Reference) (OtherComp :type Primitive%20Component%20Object%20Reference) (OtherBodyIndex :type Integer) (bFromSweep :type Boolean) (SweepResult :type Hit%20Result%20Structure%20%28by%20ref%29))
  (bind _asbp_pathway (Utilities|Casting|CastToBP_Pathway OtherActor))
  (bind _returnvalue (Game|Damage|ApplyDamage _asbp_pathway 1e+01 0 0))
  (Variables|Default|SetFridgeHealth (- (Variables|Default|GetFridgeHealth) _returnvalue))
  (Actor|DestroyActor _asbp_pathway))

(event EventBeginPlay)

(event Collision|EventActorBeginOverlap
  (params (OtherActor :type Actor%20Object%20Reference)))

(event EventTick
  (params (DeltaSeconds :type Float%20%28single-precision%29))
  (bind _fridgehealthbar (Variables|Default|GetFridgeHealthBar))
  (bind _asfridge_health_bar (Utilities|Casting|CastToFridgeHealthBar (UserInterface|GetWidget (Variables|Default|GetFridgeHealthBar))))
  (Progress|SetPercent (Variables|/Game/UI/FridgeHealthBar.FridgeHealthBar_C|GetFridgeHealthBar _asfridge_health_bar) (/ (Variables|Default|GetFridgeHealth) 1e+02))
  (Transformation|SetWorldRotation _fridgehealthbar (Math|Rotator|FindLookatRotation (Transformation|GetWorldLocation _fridgehealthbar) (Transformation|GetWorldLocation (Variables|/Script/Engine.PlayerCameraManager|GetTransformComponent (Game|GetPlayerCameraManager 0)))) false false))

(fn ConstructionScript)