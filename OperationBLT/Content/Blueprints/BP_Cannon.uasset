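; BP_Cannon is an automated turret that fires BP_CannonBall at BP_Tank enemies inside its Kill_Range.
; Overlap events maintain the enemy list; whenever the cooldown expires, Tick targets the first tank, turns toward it and fires.
; The intended closest-enemy comparison lacks an actor input and clears the target instead of reassigning it.
; The third-person character can destroy the cannon with a keypress while inside its Box.
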(event OnComponentBeginOverlap(Box)
  (params (OverlappedComponent :type Primitive%20Component%20Object%20Reference) (OtherActor :type Actor%20Object%20Reference) (OtherComp :type Primitive%20Component%20Object%20Reference) (OtherBodyIndex :type Integer) (bFromSweep :type Boolean) (SweepResult :type Hit%20Result%20Structure%20%28by%20ref%29))
  (bind _asbp_third_person_character (Utilities|Casting|CastToBP_ThirdPersonCharacter OtherActor))
  (Variables|Default|SetIs%20Inside? true))

(event OnComponentBeginOverlap(Kill_Range)
  (params (OverlappedComponent :type Primitive%20Component%20Object%20Reference) (OtherActor :type Actor%20Object%20Reference) (OtherComp :type Primitive%20Component%20Object%20Reference) (OtherBodyIndex :type Integer) (bFromSweep :type Boolean) (SweepResult :type Hit%20Result%20Structure%20%28by%20ref%29))
  ;[0.15 0.15 0.15 0.5] Adds BP_Pathways and removes from "Enemies in Range" whenever they enter/leave Kill_Range
  (bind _asbp_tank (Utilities|Casting|CastToBP_Tank OtherActor))
  (Utilities|Array|Add (Variables|Default|GetEnemiesInRange) _asbp_tank))

(event OnComponentEndOverlap(Kill_Range)
  (params (OverlappedComponent :type Primitive%20Component%20Object%20Reference) (OtherActor :type Actor%20Object%20Reference) (OtherComp :type Primitive%20Component%20Object%20Reference) (OtherBodyIndex :type Integer))
  ;[0.15 0.15 0.15 0.5] Adds BP_Pathways and removes from "Enemies in Range" whenever they enter/leave Kill_Range
  (bind _asbp_tank (Utilities|Casting|CastToBP_Tank OtherActor))
  (Utilities|Array|RemoveItem (Variables|Default|GetEnemiesInRange) _asbp_tank))

(event OnComponentEndOverlap(Box)
  (params (OverlappedComponent :type Primitive%20Component%20Object%20Reference) (OtherActor :type Actor%20Object%20Reference) (OtherComp :type Primitive%20Component%20Object%20Reference) (OtherBodyIndex :type Integer))
  (Utilities|Casting|CastToBP_ThirdPersonCharacter OtherActor)
  (Variables|Default|SetIs%20Inside? false))

(event EventTick
  (params (DeltaSeconds :type Float%20%28single-precision%29))
  (bind _enemiesinrange (Variables|Default|GetEnemiesInRange))
  (Utilities|FlowControl|Sequence
    (:then_0
      (if (<= (Variables|Default|GetCoolDown) 0.0)
        ;[0.15 0.15 0.15 0.5] Checks all enemies in range and determines which one is closest.
        (if (> (Utilities|Array|Length _enemiesinrange) 0)
          (for (_array_element _array_index) _enemiesinrange
            (bind _asbp_tank (Utilities|Casting|CastToBP_Tank _array_element)
              (:then
                ;;[0.15 0.15 0.15 0.5 10] Checks if the enemy is the first in the array and sets it to the target by default
                (if (== _array_index 0)
                  (Variables|Default|SetCurrent%20Target _asbp_tank)
                  (else
                    ;;[0.15 0.15 0.15 0.5 10] Compares how far each enemy is from the tower. Closer enemy becomes new target.
                    (if (< (Transformation|GetDistanceTo 0) (Transformation|GetDistanceTo (Variables|Default|GetCurrent%20Target)))
                      (Variables|Default|SetCurrent%20Target 0)))))
              (:CastFailed
                (Development|PrintText "CASTING ERROR! Incorrect class in targeting array! We're all gonna die!"))))
          (if (Utilities|IsValid (Variables|Default|GetCurrent%20Target))
            (Transformation|SetActorRotation (Math|Rotator|FindLookatRotation (Transformation|GetActorLocation) (Transformation|GetWorldLocation (Actor|GetComponentbyClass (Variables|Default|GetCurrent%20Target) "/Script/Engine.BoxComponent"))))
            (Game|SpawnActorfromClass "/Game/MartinFolder/BP_CannonBall.BP_CannonBall_C" (Transformation|GetWorldTransform (Variables|Default|GetArrow)) "Undefined" "MultiplyWithRoot" 0 0)
            (Variables|Default|SetCoolDown 5.0)
            (else
              (Development|PrintText "Nothing to shoot"))))))
    (:then_1
      (if (Variables|Default|GetIs%20Inside?)
        (if (Variables|/Game/Blueprints/BP_ThirdPersonCharacter.BP_ThirdPersonCharacter_C|Getkeypressed? (stale OnComponentBeginOverlap(Box) _asbp_third_person_character))
          (Actor|DestroyActor))))
    (:then_2
      (Variables|Default|SetCoolDown (- (Variables|Default|GetCoolDown) DeltaSeconds)))))

(fn ConstructionScript)