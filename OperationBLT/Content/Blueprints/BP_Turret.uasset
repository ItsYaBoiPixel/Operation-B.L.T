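; BP_Turret is a tower that automatically shoots the nearest BP_Pathway enemy within range.
; Kill_Range overlaps maintain the enemy array, which Tick scans for the closest target to face.
; A Delay on Tick paces BP_Bullet spawns from the Arrow to roughly half-second intervals.
; A Box overlap tracks the third-person character, whose Keypressed flag destroys the turret while inside.
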(event OnComponentBeginOverlap(Box)
  (params (OverlappedComponent :type Primitive%20Component%20Object%20Reference) (OtherActor :type Actor%20Object%20Reference) (OtherComp :type Primitive%20Component%20Object%20Reference) (OtherBodyIndex :type Integer) (bFromSweep :type Boolean) (SweepResult :type Hit%20Result%20Structure%20%28by%20ref%29))
  (bind _asbp_third_person_character (Utilities|Casting|CastToBP_ThirdPersonCharacter OtherActor))
  (Variables|Default|SetIsInside? true))

(event OnComponentBeginOverlap(Kill_Range)
  (params (OverlappedComponent :type Primitive%20Component%20Object%20Reference) (OtherActor :type Actor%20Object%20Reference) (OtherComp :type Primitive%20Component%20Object%20Reference) (OtherBodyIndex :type Integer) (bFromSweep :type Boolean) (SweepResult :type Hit%20Result%20Structure%20%28by%20ref%29))
  ;[0.15 0.15 0.15 0.5] Adds BP_Pathways and removes from "Enemies in Range" whenever they enter/leave Kill_Range
  (bind _asbp_pathway (Utilities|Casting|CastToBP_Pathway OtherActor))
  (Utilities|Array|Add (Variables|Default|GetEnemies_In_Range) _asbp_pathway))

(event OnComponentEndOverlap(Kill_Range)
  (params (OverlappedComponent :type Primitive%20Component%20Object%20Reference) (OtherActor :type Actor%20Object%20Reference) (OtherComp :type Primitive%20Component%20Object%20Reference) (OtherBodyIndex :type Integer))
  ;[0.15 0.15 0.15 0.5] Adds BP_Pathways and removes from "Enemies in Range" whenever they enter/leave Kill_Range
  (bind _asbp_pathway (Utilities|Casting|CastToBP_Pathway OtherActor))
  (Utilities|Array|RemoveItem (Variables|Default|GetEnemies_In_Range) _asbp_pathway))

(event OnComponentEndOverlap(Box)
  (params (OverlappedComponent :type Primitive%20Component%20Object%20Reference) (OtherActor :type Actor%20Object%20Reference) (OtherComp :type Primitive%20Component%20Object%20Reference) (OtherBodyIndex :type Integer))
  (Utilities|Casting|CastToBP_ThirdPersonCharacter OtherActor)
  (Variables|Default|SetIsInside? false))

(event EventTick
  (params (DeltaSeconds :type Float%20%28single-precision%29))
  (bind _enemies_in_range (Variables|Default|GetEnemies_In_Range))
  (Utilities|FlowControl|Sequence
    (:then_0
      ;[0.15 0.15 0.15 0.5] Checks all enemies in range and determines which one is closest.
      (if (> (Utilities|Array|Length _enemies_in_range) 0)
        (for (_array_element _array_index) _enemies_in_range
          (bind _asbp_pathway (Utilities|Casting|CastToBP_Pathway _array_element)
            (:then
              ;;[0.15 0.15 0.15 0.5 10] Checks if the enemy is the first in the array and sets it to the target by default
              (if (== _array_index 0)
                (Variables|Default|SetCurrent_Target _asbp_pathway)
                (else
                  ;;[0.15 0.15 0.15 0.5 10] Compares how far each enemy is from the tower. Closer enemy becomes new target.
                  (if (< (Transformation|GetDistanceTo _asbp_pathway) (Transformation|GetDistanceTo (Variables|Default|GetCurrent_Target)))
                    (Variables|Default|SetCurrent_Target _asbp_pathway)))))
            (:CastFailed
              (Development|PrintText "CASTING ERROR! Incorrect class in targeting array! We're all gonna die!"))))
        (if (Utilities|IsValid (Variables|Default|GetCurrent_Target))
          (Transformation|SetActorRotation (Math|Rotator|FindLookatRotation (Transformation|GetActorLocation) (Transformation|GetWorldLocation (Actor|GetComponentbyClass (Variables|Default|GetCurrent_Target) "/Script/Engine.SphereComponent"))))
          (Utilities|FlowControl|Delay 0.5)
          (Game|SpawnActorfromClass "/Game/MartinFolder/BP_Bullet.BP_Bullet_C" (Transformation|GetWorldTransform (Variables|Default|GetArrow)) "Undefined" "MultiplyWithRoot" 0 0)
          (else
            (Development|PrintText "Nothing to shoot")))))
    (:then_1
      (if (Variables|Default|GetIsInside?)
        (if (Variables|/Game/Blueprints/BP_ThirdPersonCharacter.BP_ThirdPersonCharacter_C|Getkeypressed? (stale OnComponentBeginOverlap(Box) _asbp_third_person_character))
          (Actor|DestroyActor))))))

(fn ConstructionScript)