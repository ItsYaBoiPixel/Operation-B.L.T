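; BP_Pathway is an actor that moves a Walker component endlessly along a spline path.
; A timeline, with its play rate set from Speed, maps alpha to distance along the spline and sets the Walker's world location and rotation.
; When the timeline finishes, the walk restarts from the beginning of the spline.
; Overlap of EnemyCollision with a BP_Fridge destroys that collision component.
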(event OnComponentBeginOverlap(EnemyCollision)
  (params (OverlappedComponent :type Primitive%20Component%20Object%20Reference) (OtherActor :type Actor%20Object%20Reference) (OtherComp :type Primitive%20Component%20Object%20Reference) (OtherBodyIndex :type Integer) (bFromSweep :type Boolean) (SweepResult :type Hit%20Result%20Structure%20%28by%20ref%29))
  (Utilities|Casting|CastToBP_Fridge OtherActor)
  (Components|DestroyComponent (Variables|Default|GetEnemyCollision)))

(event Custom|Walk
  (Components|Timeline|SetPlayRate (Variables|Default|GetWalkTimeline) (Variables|Default|GetSpeed))
  (bind _walktrack (Timeline|WalkTimeline PlayFromStart)
    (:Update
      (Transformation|SetWorldLocationAndRotation (Variables|Default|GetWalker) (.location (Spline|GetTransformatDistanceAlongSpline (Variables|Default|GetSpline) (Math|Float|Lerp 0.0 (Spline|GetSplineLength (Variables|Default|GetSpline)) _walktrack) "World" false)) (.rotation (Spline|GetTransformatDistanceAlongSpline (Variables|Default|GetSpline) (Math|Float|Lerp 0.0 (Spline|GetSplineLength (Variables|Default|GetSpline)) _walktrack) "World" false)) false false))
    (:Finished
      (CallFunction|Walk))))

(event EventBeginPlay
  (CallFunction|Walk))

(event Collision|EventActorBeginOverlap
  (params (OtherActor :type Actor%20Object%20Reference)))

(event EventTick
  (params (DeltaSeconds :type Float%20%28single-precision%29)))

(fn ConstructionScript)