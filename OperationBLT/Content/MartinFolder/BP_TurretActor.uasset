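; Turret actor that locks onto "Enemy"-tagged actors entering its detection sphere.
; Overlap stores the target and starts two looping timers: one yaws the turret mesh toward it, the other line-traces at it from above the actor origin.
; The trace checks for an Enemy hit but applies no effect yet.
; A tagged actor leaving the sphere clears both timers while the target is valid.
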(event OnComponentBeginOverlap(Sphere)
  (params (OverlappedComponent :type Primitive%20Component%20Object%20Reference) (OtherActor :type Actor%20Object%20Reference) (OtherComp :type Primitive%20Component%20Object%20Reference) (OtherBodyIndex :type Integer) (bFromSweep :type Boolean) (SweepResult :type Hit%20Result%20Structure%20%28by%20ref%29))
  ;[0.15 0.15 0.15 0.5] When See Enemy, Set Target
  (Utilities|IsValid OtherActor
    (:Is%20Valid
      (if (Actor|ActorHasTag OtherActor "Enemy")
        (Variables|Default|SetTarget OtherActor)
        (CallFunction|TrackTarget)))))

(event OnComponentEndOverlap(Sphere)
  (params (OverlappedComponent :type Primitive%20Component%20Object%20Reference) (OtherActor :type Actor%20Object%20Reference) (OtherComp :type Primitive%20Component%20Object%20Reference) (OtherBodyIndex :type Integer))
  ;[0.15 0.15 0.15 0.5] When Player Leaves Range, Stop Tracking
  (Utilities|IsValid OtherActor
    (:Is%20Valid
      (if (Actor|ActorHasTag OtherActor "Enemy")
        (Variables|Default|GetTarget
          (:then
            (Utilities|Time|ClearandInvalidateTimerbyHandle (Variables|Default|GetTimerRef))
            (Utilities|Time|ClearandInvalidateTimerbyHandle (Variables|Default|GetFireTimer)))
          (:else))))))

(event Custom|TrackTarget
  ;[0.15 0.15 0.15 0.5] Rotate Turret
  (bind _returnvalue (Utilities|Time|SetTimerbyEvent (delegate Custom|MoveTurret) 0.05 true true))
  (Variables|Default|SetTimerRef _returnvalue)
  (bind _returnvalue_2 (Utilities|Time|SetTimerbyEvent (delegate Custom|ShootTurret) 0.3 true true))
  (Variables|Default|SetFireTimer _returnvalue_2))

(event Custom|MoveTurret
  (bind _target (Variables|Default|GetTarget))
  ;[0.15 0.15 0.15 0.5] Rotate Turret
  (Utilities|IsValid _target
    (:Is%20Valid
      (Transformation|SetRelativeRotation (Variables|Default|GetMDL_Turret) (Math|Rotator|MakeRotator 0.0 0.0 (.yaw (Math|Interpolation|RInterpTo (Variables|/Script/Engine.SceneComponent|GetRelativeRotation (Variables|Default|GetMDL_Turret)) (Math|Rotator|FindLookatRotation (Transformation|GetActorLocation) (Transformation|GetActorLocation _target)) (Utilities|Time|GetWorldDeltaSeconds) 1e+02))) false false))))

(event Custom|ShootTurret
  ;[0.15 0.15 0.15 0.5] Fire Line Trace, See If Hit Player
  (bind (_outhit _returnvalue) (Collision|LineTraceByChannel (+ (Transformation|GetActorLocation) "0.000000,0.000000,80.000000") (Transformation|GetActorLocation (Variables|Default|GetTarget)) "TraceTypeQuery1" false 0 "None"))
  (if _returnvalue
    (if (Actor|ActorHasTag (.HitActor (Collision|BreakHitResult _outhit)) "Enemy")
      _)))

(fn ConstructionScript)