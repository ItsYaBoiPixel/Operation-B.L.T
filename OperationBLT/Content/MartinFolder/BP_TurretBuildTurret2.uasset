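; BP_TurretBuildTurret2 appears to be a turret build display with a floating scrap price.
; Every Tick, ShowThis selects the visuals: a value of 2 shows the Cylinder at 75 scrap, any other value shows two instanced static mesh components at 150 scrap.
; Tick also rotates the Price text to face the player camera.
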(event EventBeginPlay)

(event Collision|EventActorBeginOverlap
  (params (OtherActor :type Actor%20Object%20Reference)))

(event EventTick
  (params (DeltaSeconds :type Float%20%28single-precision%29))
  (bind _price (Variables|Default|GetPrice))
  (Utilities|FlowControl|Sequence
    (:then_0
      (switch int (Variables|Default|GetShowThis)
        (:Default
          (Rendering|SetVisibility (Variables|Default|GetCylinder) false true :!label _label)
          (Rendering|SetVisibility (Variables|Default|GetHierarchicalInstancedStaticMesh) true true)
          (Rendering|Components|TextRender|SetText (Variables|Default|GetPrice) (Utilities|Text|MakeLiteralText "150 scrap")))
        (:0
          (goto _label))
        (:1
          (goto _label))
        (:2
          (Rendering|SetVisibility (Variables|Default|GetCylinder) true true)
          (Rendering|SetVisibility (Variables|Default|GetHierarchicalInstancedStaticMesh) false true)
          (Rendering|Components|TextRender|SetText (Variables|Default|GetPrice) (Utilities|Text|MakeLiteralText "75 scrap")))))
    (:then_1
      (Transformation|SetWorldRotation _price (Math|Rotator|FindLookatRotation (Transformation|GetWorldLocation _price) (Transformation|GetWorldLocation (Variables|/Script/Engine.PlayerCameraManager|GetTransformComponent (Game|GetPlayerCameraManager 0)))) false false))))

(fn ConstructionScript)

(fn NewFunction)